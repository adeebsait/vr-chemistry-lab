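; BP_Dish is a lab dish that runs chemical reactions on the molecules it holds.
; Reactions scans every D_Reactions data table row, using CheckContent and CheckQuantity to confirm each input molecule is present and strictly exceeds the required amount.
; Matching rows remove their inputs through MoleculesRemove, then add their outputs through MoleculesAdd, so recipes are data-driven.
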(fn ConstructionScript)

(fn Reactions
  (bind _outrownames (DataTable|GetDataTableRowNames "/Game/LAB/DataTables/D_Reactions.D_Reactions"))
  (for _array_element _outrownames
    (bind _returnvalue (Utilities|GetDataTableRow "/Game/LAB/DataTables/D_Reactions.D_Reactions" _array_element)
      (:then
        (bind _keys (Utilities|Map|Keys "NewEnumerator0"))
        (bind _keys_2 (Utilities|Map|Keys (.Input (Utilities|Struct|BreakF_Reactions _returnvalue))))
        (bind _return1 (CallFunction|CheckContent _keys _keys_2))
        (bind _result (CallFunction|CheckQuantity (.Input (Utilities|Struct|BreakF_Reactions _returnvalue))))
        (if (and _return1 _result)
          (Utilities|FlowControl|Sequence
            (:then_0
              (bind _keys_3 (Utilities|Map|Keys (.Input (Utilities|Struct|BreakF_Reactions _returnvalue))))
              (for _array_element_2 _keys_3
                (CallFunction|MoleculesRemove (.Value (Utilities|Map|Find (.Input (Utilities|Struct|BreakF_Reactions _returnvalue)) _array_element_2)) _array_element_2)))
            (:then_1
              (bind _keys_4 (Utilities|Map|Keys (.Output (Utilities|Struct|BreakF_Reactions _returnvalue))))
              (for _array_element_3 _keys_4
                (CallFunction|MoleculesAdd (.Value (Utilities|Map|Find (.Output (Utilities|Struct|BreakF_Reactions _returnvalue)) _array_element_3)) _array_element_3)))))))))

(fn CheckContent
  (params (Array :type Array%20of%20EMolecules%20Enums :default "NewEnumerator0") (Array1 :type Array%20of%20EMolecules%20Enums :default "NewEnumerator0"))
  (for _array_element Array1
    (if (not (Utilities|Array|ContainsItem Array _array_element))
      (return false)))
  (return true))

(fn CheckQuantity
  (params (TargetMap :type Map%20of%20EMolecules%20Enums%20to%20Reals :default "NewEnumerator0"))
  (bind _keys (Utilities|Map|Keys TargetMap))
  (for _array_element _keys
    (if (<= (.Value (Utilities|Map|Find "NewEnumerator0" _array_element)) (.Value (Utilities|Map|Find TargetMap _array_element)))
      (return false)))
  (return true))