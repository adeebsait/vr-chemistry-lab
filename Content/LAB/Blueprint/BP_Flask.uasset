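; Lab flask that holds a map of molecule amounts and simulates their mixing, gas escape and chemical reactions.
; Each tick it lets gases escape, totals the contents and computes pH and color as amount-weighted averages of non-gas molecules from D_Molecules.
; Reactions from D_Reactions swap inputs for outputs when enough is present.
; An interpolated fill level scales the liquid mesh, tinted through a cached dynamic material, with optional debug text.
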(event Custom|UpdateLiquidScale
  (bind _liquid (Variables|Default|GetLiquid))
  ;[1 1 1] UpdateLiquidScale
  (if (== (Variables|Default|Getliquid_visual) 0.0)
    (Rendering|SetVisibility _liquid false false)
    (Transformation|SetRelativeScale3D _liquid (Math|Vector|MakeVector 0.0 0.0 0.0))
    (else
      (Rendering|SetVisibility _liquid true false)
      (Transformation|SetRelativeScale3D _liquid (Math|Vector|MakeVector 1.0 1.0 (Math|Interpolation|Ease "Linear" (/ (Variables|Default|Getliquid_visual) (Variables|Default|Getliquid_max)) 0.1 0.87))))))

(event Custom|MoleculesRemove
  (params (liquid :type Float%20%28double-precision%29) (Key :type EMolecules%20Enum%20%28by%20ref%29 :default "NewEnumerator0"))
  ;[1 1 1] MoleculesRemove
  (if (Utilities|Map|Contains (Variables|Default|Getmolecules) Key)
    (CallFunction|MoleculesAdd (* liquid -1.0) Key)))

(event Custom|UpdateColor
  ;[1 1 1] UpdateColor
  (Rendering|Material|SetVectorParameterValue (Variables|Default|Getliquid_material) "Color" (Variables|Default|Getcolor) :!class /Script/Engine.MaterialInstanceDynamic))

(event Custom|MoleculesAdd
  (params (liquid :type Float%20%28double-precision%29) (Key :type EMolecules%20Enum%20%28by%20ref%29 :default "NewEnumerator0"))
  (bind _molecules (Variables|Default|Getmolecules))
  (bind _returnvalue (Utilities|Map|Contains _molecules Key))
  (bind _value (Utilities|Map|Find _molecules Key))
  (bind _returnvalue_2 (+ _value liquid))
  (bind _returnvalue_3 (Math|Float|SelectFloat _returnvalue_2 liquid _returnvalue))
  ;[1 1 1] MoleculesAdd
  (if (< (Variables|Default|Getliquid_total) (Variables|Default|Getliquid_max))
    (Utilities|Map|Add _molecules Key _returnvalue_3)
    (if (== (Math|Float|Clamp(Float) _returnvalue_3 0.0 (Variables|Default|Getliquid_max)) 0.0)
      (Utilities|Map|Remove (Variables|Default|Getmolecules) Key))))

(event EventBeginPlay
  ;[1 1 1] Store dynamic material instance in variable to fast reuse instead of creating more
  (bind _returnvalue (Rendering|Material|CreateDynamicMaterialInstance (Variables|Default|GetLiquid) 0 "/Game/LAB/Material/instances/MI_Lab_Inst.MI_Lab_Inst" "None" :!class /Script/Engine.PrimitiveComponent))
  (Variables|Default|Setliquid_material _returnvalue))

(event Collision|EventActorBeginOverlap
  (params (OtherActor :type Actor%20Object%20Reference)))

(event EventTick
  (params (DeltaSeconds :type Float%20%28single-precision%29))
  ;[1 1 1] Tick (Gas scape, total calculation, ph, color, reactions, debug)
  (Utilities|FlowControl|Sequence
    (:then_0
      (|GasScape))
    (:then_1
      (|Sumtotalcontent))
    (:then_2
      (|Calculatephandcolor))
    (:then_3
      ;;[1 1 1] Debug, change the Debug variable to True/False
      (if (Variables|Default|Getdebug)
        (|DebugNodes)))
    (:then_5
      ;;[1 1 1] Final
      (Variables|Default|Setliquid_visual (Math|Interpolation|FInterpTo (Variables|Default|Getliquid_visual) (Variables|Default|Getliquid_total) DeltaSeconds 5.0))
      (CallFunction|UpdateLiquidScale)
      (CallFunction|UpdateColor)
      (CallFunction|Reactions))))

(fn ConstructionScript)

(fn Reactions
  (bind _outrownames (DataTable|GetDataTableRowNames "/Game/LAB/DataTables/D_Reactions.D_Reactions"))
  (for _array_element _outrownames
    (bind _returnvalue (Utilities|GetDataTableRow "/Game/LAB/DataTables/D_Reactions.D_Reactions" _array_element)
      (:then
        (bind _keys (Utilities|Map|Keys (Variables|Default|Getmolecules)))
        (bind _keys_2 (Utilities|Map|Keys (.Input (Utilities|Struct|BreakF_Reactions _returnvalue))))
        (bind _return1 (CallFunction|CheckContent _keys _keys_2))
        (bind _result (CallFunction|CheckQuantity (.Input (Utilities|Struct|BreakF_Reactions _returnvalue))))
        (if (and _return1 _result)
          (Utilities|FlowControl|Sequence
            (:then_0
              (bind _keys_3 (Utilities|Map|Keys (.Input (Utilities|Struct|BreakF_Reactions _returnvalue))))
              (for _array_element_2 _keys_3
                (CallFunction|MoleculesRemove (.Value (Utilities|Map|Find (.Input (Utilities|Struct|BreakF_Reactions _returnvalue)) _array_element_2)) _array_element_2)))
            (:then_1
              (bind _keys_4 (Utilities|Map|Keys (.Output (Utilities|Struct|BreakF_Reactions _returnvalue))))
              (for _array_element_3 _keys_4
                (CallFunction|MoleculesAdd (.Value (Utilities|Map|Find (.Output (Utilities|Struct|BreakF_Reactions _returnvalue)) _array_element_3)) _array_element_3)))))))))

(fn CheckContent
  (params (Array :type Array%20of%20EMolecules%20Enums :default "NewEnumerator0") (Array1 :type Array%20of%20EMolecules%20Enums :default "NewEnumerator0"))
  (for _array_element Array1
    (if (not (Utilities|Array|ContainsItem Array _array_element))
      (return false)))
  (return true))

(fn CheckQuantity
  (params (TargetMap :type Map%20of%20EMolecules%20Enums%20to%20Reals :default "NewEnumerator0"))
  (bind _keys (Utilities|Map|Keys TargetMap))
  (for _array_element _keys
    (if (<= (.Value (Utilities|Map|Find (Variables|Default|Getmolecules) _array_element)) (.Value (Utilities|Map|Find TargetMap _array_element)))
      (return false)))
  (return true))