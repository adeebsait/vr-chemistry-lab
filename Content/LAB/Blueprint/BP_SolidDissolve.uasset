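; BP_SolidDissolve is a lab solid that dissolves while overlapping a beaker (BP_Becher).
; Mesh overlap events set and clear the target beaker.
; Each tick it scales the actor by MassPercentage, shrinks that percentage at an accelerating rate, and adds a fixed fraction of OriginalMass to the beaker as molecules of its Type.
; It destroys itself below DisappearPercentage and can show the percentage as debug text.
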(event OnComponentHit(StaticMeshComponent)
  (params (HitComponent :type Primitive%20Component%20Object%20Reference) (OtherActor :type Actor%20Object%20Reference) (OtherComp :type Primitive%20Component%20Object%20Reference) (NormalImpulse :type Vector :default "0, 0, 0") (Hit :type Hit%20Result%20Structure%20%28by%20ref%29)))

(event OnComponentBeginOverlap(StaticMeshComponent)
  (params (OverlappedComponent :type Primitive%20Component%20Object%20Reference) (OtherActor :type Actor%20Object%20Reference) (OtherComp :type Primitive%20Component%20Object%20Reference) (OtherBodyIndex :type Integer) (bFromSweep :type Boolean) (SweepResult :type Hit%20Result%20Structure%20%28by%20ref%29))
  ;[1 1 1] Update DissolveTo
  (bind _asbp_becher (Utilities|Casting|CastToBP_Becher OtherActor))
  (Variables|Default|Setdissolve_to _asbp_becher))

(event OnComponentEndOverlap(StaticMeshComponent)
  (params (OverlappedComponent :type Primitive%20Component%20Object%20Reference) (OtherActor :type Actor%20Object%20Reference) (OtherComp :type Primitive%20Component%20Object%20Reference) (OtherBodyIndex :type Integer))
  ;[1 1 1] Clear DissolveTo
  (Variables|Default|Setdissolve_to 0))

(event EventBeginPlay)

(event Collision|EventActorBeginOverlap
  (params (OtherActor :type Actor%20Object%20Reference)))

(event EventTick
  (params (DeltaSeconds :type Float%20%28single-precision%29))
  (bind _debugtext (Variables|Default|GetDebugText))
  (Utilities|FlowControl|Sequence
    (:then_0
      ;[1 1 1] Dissolve
      (Transformation|SetActorScale3D (Math|Conversions|ToVector(Float) (Variables|Default|Getmass_percentage)))
      (bind _dissolve_to (Variables|Default|Getdissolve_to)
        (:then
          (Variables|Default|Setmass_percentage (- (Variables|Default|Getmass_percentage) (* 0.005 (- 2.0 (Variables|Default|Getmass_percentage)))))
          (Default|MoleculesAdd _dissolve_to (* (/ (Variables|Default|Getoriginal_mass) 1e+02) 0.884956) (Variables|Default|Gettype)))
        (:else)))
    (:then_1
      ;[1 1 1] Debug
      (if (Variables|Default|GetDebug)
        (Rendering|Components|TextRender|SetText _debugtext (Utilities|Text|ToText(Float) (Variables|Default|Getmass_percentage) "HalfToEven"))
        (Rendering|SetVisibility _debugtext true false)))
    (:then_3
      ;[1 1 1] destroy before becoming almost invisible
      (if (< (Variables|Default|Getmass_percentage) (Variables|Default|Getdisappear_percentage))
        (Actor|DestroyActor)))))

(fn ConstructionScript)