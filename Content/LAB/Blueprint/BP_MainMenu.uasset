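; BP_MainMenu is the VR main menu Blueprint, handling laser-pointer aiming and clicking for UI interaction.
; Each tick it feeds a fixed-length line from the VRPawn's right WidgetInteraction component into the MenuLaser Niagara system's point array to draw the laser.
; Either trigger presses and releases a simulated left mouse button on that same right-hand component, so the left trigger also clicks where the right hand points.
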(event EventBeginPlay)

(event Collision|EventActorBeginOverlap
  (params (OtherActor :type Actor%20Object%20Reference)))

(event EventTick
  (params (DeltaSeconds :type Float%20%28single-precision%29))
  (bind _menulaser (Variables|Default|GetMenuLaser))
  ;[1 1 1] Draw Laser
  (bind _asvrpawn (Utilities|Casting|CastToVRPawn (Game|Player|GetPlayerPawn 0)))
  (Class|NiagaraDataInterfaceArrayFunctionLibrary|SetNiagaraArrayVectorValue _menulaser "User.PointArray" 0 (Transformation|GetWorldLocation (Variables|/Game/VRTemplate/Blueprints/VRPawn.VRPawn_C|GetWidgetInteractionRight _asvrpawn)) false) ; MenuLaser start location
  (Class|NiagaraDataInterfaceArrayFunctionLibrary|SetNiagaraArrayVectorValue _menulaser "User.PointArray" 1 (+ (Transformation|GetWorldLocation (Variables|/Game/VRTemplate/Blueprints/VRPawn.VRPawn_C|GetWidgetInteractionRight _asvrpawn)) (* (Math|Vector|GetForwardVector (Variables|/Game/VRTemplate/Blueprints/VRPawn.VRPawn_C|GetWidgetInteractionRight _asvrpawn)) (Math|Float|MakeLiteralFloat 5e+02))) false) ; MenuLaser end location
)

(event Input|ActionEvents|InputActionTriggerLeft
  (params (Key :type Key%20Structure :default "None"))
  (bind _returnvalue (Game|Player|GetPlayerPawn 0))
  ;[1 1 1] Click with Trigger
  (:Pressed
    (bind _asvrpawn (Utilities|Casting|CastToVRPawn _returnvalue))
    (Class|WidgetInteractionComponent|PressPointerKey (Variables|/Game/VRTemplate/Blueprints/VRPawn.VRPawn_C|GetWidgetInteractionRight _asvrpawn) "LeftMouseButton"))
  (:Released
    (bind _asvrpawn_2 (Utilities|Casting|CastToVRPawn _returnvalue))
    (Class|WidgetInteractionComponent|ReleasePointerKey (Variables|/Game/VRTemplate/Blueprints/VRPawn.VRPawn_C|GetWidgetInteractionRight _asvrpawn_2) "LeftMouseButton")))

(event Input|ActionEvents|InputActionTriggerRight
  (params (Key :type Key%20Structure :default "None"))
  (bind _returnvalue (Game|Player|GetPlayerPawn 0))
  ;[1 1 1] Click with Trigger
  (:Pressed
    (bind _asvrpawn (Utilities|Casting|CastToVRPawn _returnvalue))
    (Class|WidgetInteractionComponent|PressPointerKey (Variables|/Game/VRTemplate/Blueprints/VRPawn.VRPawn_C|GetWidgetInteractionRight _asvrpawn) "LeftMouseButton"))
  (:Released
    (bind _asvrpawn_2 (Utilities|Casting|CastToVRPawn _returnvalue))
    (Class|WidgetInteractionComponent|ReleasePointerKey (Variables|/Game/VRTemplate/Blueprints/VRPawn.VRPawn_C|GetWidgetInteractionRight _asvrpawn_2) "LeftMouseButton")))

(fn ConstructionScript)