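; BP_phMeter is a lab pH meter actor that changes color when it overlaps a beaker (BP_Becher) containing liquid.
; On BeginPlay it creates a dynamic material instance on its static mesh and sets it to white.
; On overlap with a non-empty beaker, it maps the beaker's pH on the 14-point scale linearly to an HSV hue and writes that color to the material.
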(event OnComponentBeginOverlap(StaticMeshComponent)
  (params (OverlappedComponent :type Primitive%20Component%20Object%20Reference) (OtherActor :type Actor%20Object%20Reference) (OtherComp :type Primitive%20Component%20Object%20Reference) (OtherBodyIndex :type Integer) (bFromSweep :type Boolean) (SweepResult :type Hit%20Result%20Structure%20%28by%20ref%29))
  ;[1 1 1] Change color by Overlap with Becher
  (bind _asbp_becher (Utilities|Casting|CastToBP_Becher OtherActor))
  (if (> (Variables|/Game/LAB/Blueprint/BP_Becher.BP_Becher_C|Getliquid_visual _asbp_becher) 0.0)
    (Rendering|Material|SetVectorParameterValue (Variables|Default|Getmaterial) "Color" (Class|KismetMathLibrary|HSVtoRGB (Math|Interpolation|Ease "Linear" (/ (Variables|/Game/LAB/Blueprint/BP_Becher.BP_Becher_C|GetpH _asbp_becher) 14.0) 0.0 2.6e+02) 1.0 1.0 1.0) :!class /Script/Engine.MaterialInstanceDynamic)))

(event EventBeginPlay
  (bind _returnvalue (Rendering|Material|CreateDynamicMaterialInstance (Variables|Debug|GetStaticMeshComponent) 0 "/Game/LAB/Material/instances/MI_Lab_Inst.MI_Lab_Inst" "None" :!class /Script/Engine.PrimitiveComponent))
  (bind _output_get (Variables|Default|Setmaterial _returnvalue))
  (Rendering|Material|SetVectorParameterValue _output_get "Color" "(R=1.000000,G=1.000000,B=1.000000,A=1.000000)" :!class /Script/Engine.MaterialInstanceDynamic))

(event Collision|EventActorBeginOverlap
  (params (OtherActor :type Actor%20Object%20Reference)))

(event EventTick
  (params (DeltaSeconds :type Float%20%28single-precision%29)))

(fn ConstructionScript)