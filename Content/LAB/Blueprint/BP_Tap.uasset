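; Lab tap actor that dispenses its configured liquid type into beakers placed beneath it.
; On BeginPlay it looks up the type in the D_Molecules table, then sets its label's text and color and offsets itself locally.
; Every Tick a capsule trace runs down from the mesh's Drop socket, adding Flow of that liquid to any BP_Becher hit, without delta-time scaling.
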(event EventBeginPlay
  (bind _liquid_type (Variables|Default|GetLiquid%20Type))
  (bind _returnvalue (Utilities|String|EnumtoString _liquid_type))
  ;[1 1 1] Change text color and add offset
  (bind _returnvalue_2 (Utilities|GetDataTableRow "/Game/LAB/DataTables/D_Molecules.D_Molecules" (Utilities|String|StringToName _returnvalue))
    (:then
      (Rendering|Components|TextRender|SetText (Variables|Default|GetTextRender) (Utilities|Text|ToText(String) _returnvalue))
      (Rendering|Components|TextRender|SetTextRenderColor (Variables|Default|GetTextRender) (Math|Conversions|ToColor(LinearColor) (.Color (Utilities|Struct|BreakF_Molecules _returnvalue_2))))
      (Transformation|AddActorLocalOffset "-40.000000,0.000000,33.000000" false false))))

(event Collision|EventActorBeginOverlap
  (params (OtherActor :type Actor%20Object%20Reference)))

(event EventTick
  (params (DeltaSeconds :type Float%20%28single-precision%29))
  (bind _staticmeshcomponent (Variables|Debug|GetStaticMeshComponent))
  (bind _returnvalue (Transformation|GetSocketLocation _staticmeshcomponent "Drop"))
  (bind (_outhit _returnvalue_2) (Collision|CapsuleTraceByChannel _returnvalue (- _returnvalue "0,0,100.000000") 2.0 13.0 "TraceTypeQuery1" false 0 "None"))
  (if _returnvalue_2
    (bind _asbp_becher (Utilities|Casting|CastToBP_Becher (.HitActor (Collision|BreakHitResult _outhit))))
    (Default|MoleculesAdd _asbp_becher (Variables|Default|GetFlow) (Variables|Default|GetLiquid%20Type))))

(fn ConstructionScript)